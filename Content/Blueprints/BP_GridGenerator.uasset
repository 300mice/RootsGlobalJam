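; BP_GridGenerator spawns a randomized grid of BP_Node actors when play begins.
; Nested loops over YSize and XSize place nodes at multiples of GridDistance along world X and Y, independent of the generator's own location.
; Each cell has a one-in-four chance of being left empty, producing irregular gaps in the grid.
; The click event on Nodes is an empty stub.
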(event `self.ReceiveBeginPlay`
  (for _index (range (+ (`self.YSize`) 1))
    (for _index_2 (range (+ (`self.XSize`) 1))
      (if (not (== (`KismetMathLibrary.RandomIntegerInRange` 0 3) 0))
        (`|SpawnActorFromClass` "/Game/Blueprints/BP_Node.BP_Node_C" (`KismetMathLibrary.MakeTransform` (`KismetMathLibrary.MakeVector` (* _index_2 (`self.GridDistance`)) (* _index (`self.GridDistance`)))) "Undefined" "OverrideRootScale" null null)))))

(event `self.Nodes.OnClicked`
  (params (TouchedComponent :type "PrimitiveComponent Object Reference") (ButtonPressed :type "Key Structure")))

(fn `UserConstructionScript`)