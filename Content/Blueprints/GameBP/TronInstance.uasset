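; Game instance Blueprint that hosts, joins, updates and destroys multiplayer sessions through Advanced Sessions nodes.
; Hosting tags the session with a random SessionName and a GameStarted flag, then opens the test level as a listen server; lobby and in-progress events update that flag.
; For new joins, RefreshServer_2 searches again and matches SessionName to get current settings, so joining proceeds only if the game has not started.
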(event `HostSession`
  (params (NumberOfPlayers :type Integer))
  (bind _output_get (set `self.SessionName` (`KismetStringLibrary.Concat_StrStr` "game" (`KismetStringLibrary.Conv_Int64ToString` (`KismetMathLibrary.RandomInteger64` 999999999)))))
  (`KismetSystemLibrary.PrintString` _output_get true true (struct :`G` 0.66 :`B` 1.0 :`A` 1.0) 150.0)
  (set `self.Number Of Players` NumberOfPlayers)
  (`KismetSystemLibrary.PrintString` "Hello")
  (`CreateSessionCallbackProxyAdvanced.CreateAdvancedSession` (`|MakeArray` (`AdvancedSessionsLibrary.MakeLiteralSessionPropertyBool` "GameStarted") (`AdvancedSessionsLibrary.MakeLiteralSessionPropertyString` "SessionName" (`self.SessionName`))) (`GameplayStatics.GetPlayerController` 0) 4
    (:`OnSuccess`
      (`GameplayStatics.OpenLevelBySoftObjectPtr` "/Game/Levels/TestLevel.TestLevel" true "listen")
      (`KismetSystemLibrary.PrintString` "Hosting!"))
    (:`OnFailure`
      (`KismetSystemLibrary.PrintString` "Failed Host" true true (struct :`R` 1.0 :`A` 1.0)))))

(event `DestroySession`
  (`DestroySessionCallbackProxy.DestroySession` (`GameplayStatics.GetPlayerController` 0)
    (:`OnSuccess`
      (`KismetSystemLibrary.PrintString` "DestroyOldSession"))))

(event `SessionInProgress`
  (`UpdateSessionCallbackProxyAdvanced.UpdateSession` (`|MakeArray` (`AdvancedSessionsLibrary.MakeLiteralSessionPropertyBool` "GameStarted" true) (`AdvancedSessionsLibrary.MakeLiteralSessionPropertyString` "SessionName" (`self.SessionName`))) 4 0 false true true
    (:`OnSuccess`
      (`KismetSystemLibrary.PrintString` "StartedGame" true true (struct :`R` 0.530492 :`G` 0.383302 :`B` 1.0 :`A` 1.0) 50.0))))

(event `Join Session`
  (params (Session :type "BlueprintSessionResult Structure") (New :type Boolean))
  ;[1 1 1] Joining an existing session
  (if New
    (bind _extrasettings (`AdvancedSessionsLibrary.GetExtraSettings` Session))
    (bind _settingvalue (`AdvancedSessionsLibrary.GetSessionPropertyString` _extrasettings "SessionName")
      (:`Found`
        (bind _results (`FindSessionsCallbackProxyAdvanced.FindSessionsAdvanced` (`GameplayStatics.GetPlayerController` 0) 10 false "AllServers")
          (:`OnSuccess`
            (for _array_element _results
              (bind _extrasettings_2 (`AdvancedSessionsLibrary.GetExtraSettings` _array_element))
              (bind _settingvalue_2 (`AdvancedSessionsLibrary.GetSessionPropertyString` _extrasettings_2 "SessionName")
                (:`Found`
                  (if (`KismetStringLibrary.EqualEqual_StrStr` _settingvalue_2 _settingvalue)
                    (bind _extrasettings_3 (`AdvancedSessionsLibrary.GetExtraSettings` _array_element))
                    (bind _settingvalue_3 (`AdvancedSessionsLibrary.GetSessionPropertyBool` _extrasettings_3 "GameStarted")
                      (:`Found`
                        (if (not _settingvalue_3)
                          (`JoinSessionCallbackProxy.JoinSession` (`GameplayStatics.GetPlayerController` 0) Session :!label _label
                            (:`OnSuccess`
                              (bind _extrasettings_4 (`AdvancedSessionsLibrary.GetExtraSettings` Session))
                              (bind _settingvalue_4 (`AdvancedSessionsLibrary.GetSessionPropertyString` _extrasettings_4 "SessionName")
                                (:`Found`
                                  (bind _output_get (set `self.SessionName` _settingvalue_4))
                                  (`KismetSystemLibrary.PrintString` _output_get true true (struct :`R` 1.0 :`G` 0.138286 :`A` 1.0) 150.0))))))))))))))))
    (else
      (goto _label))))

(event `SessionInLobby`
  (`UpdateSessionCallbackProxyAdvanced.UpdateSession` (`|MakeArray` (`AdvancedSessionsLibrary.MakeLiteralSessionPropertyBool` "GameStarted") (`AdvancedSessionsLibrary.MakeLiteralSessionPropertyString` "SessionName" (`self.SessionName`))) 4 0 false true true
    (:`OnSuccess`
      (`KismetSystemLibrary.PrintString` "ServerUpdated" true true (struct :`R` 0.608835 :`G` 1.0 :`B` 0.417691 :`A` 1.0) 50.0))))