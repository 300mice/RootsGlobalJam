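; Player pawn that drives an orthographic camera for viewing a BP_GridGenerator grid and creates the HUD on begin play.
; Zoom and pan input set targets that Tick smoothly interpolates toward, with Space recentering on the grid.
; Zoom limits, zoom step and pan speed derive from grid size.
; Once movement settles, the target clamps to bounds around the grid center that widen as the camera zooms in.
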(event `self.ReceiveBeginPlay`
  (bind _returnvalue (`GameplayStatics.GetActorOfClass` "/Game/Blueprints/BP_GridGenerator.BP_GridGenerator_C"))
  (set `self.Grid` _returnvalue)
  (set `self.ZoomIncrement` (/ (`self.GetGridSize`) 2.0))
  (bind _returnvalue_2 (`|CreateWidget` "/Game/UI/W_HUD.W_HUD_C"))
  (`UserWidget.AddToViewport` _returnvalue_2 0)
  (set `self.MoveSpeed` (`KismetMathLibrary.Sqrt` (`self.GetGridSize`))))

(event `self.ReceiveTick`
  (params (DeltaSeconds :type "Float (single-precision)"))
  (bind _returnvalue (`self.GetGridSize`))
  (bind (_returnvalue_x _returnvalue_y) (`KismetMathLibrary.BreakVector` (`self.K2_GetActorLocation`)))
  (bind _returnvalue_2 (`self.GetGridSize`))
  (bind (_output_get_x _output_get_y) (`KismetMathLibrary.BreakVector` (`self.GetGridCenter`)))
  (bind _returnvalue_3 (* (+ (* (`KismetMathLibrary.NormalizeToRange` (`CameraComponent.OrthoWidth` (`self.Camera`)) (/ _returnvalue 5.0) _returnvalue) -1.0) 1.0) (/ (`self.GetGridSize`) 4.0)))
  (`CameraComponent.SetOrthoWidth` (`self.Camera`) (`KismetMathLibrary.FClamp` (`KismetMathLibrary.FInterpTo` (`CameraComponent.OrthoWidth` (`self.Camera`)) (`self.TargetZoom`) (`GameplayStatics.GetWorldDeltaSeconds`) 5.0) (/ _returnvalue_2 4.0) _returnvalue_2))
  (`self.K2_SetActorLocation` (`KismetMathLibrary.VInterpTo` (`self.K2_GetActorLocation`) (`self.TargetLocation`) (`GameplayStatics.GetWorldDeltaSeconds`) 4.0))
  (if (not (!= (`self.K2_GetActorLocation`) (`self.TargetLocation`) :`ErrorTolerance` 10.0))
    (set `self.TargetLocation` (`KismetMathLibrary.MakeVector` (`KismetMathLibrary.FClamp` _returnvalue_x (- _output_get_x _returnvalue_3) (+ _returnvalue_3 _output_get_x)) (`KismetMathLibrary.FClamp` _returnvalue_y (- _output_get_y _returnvalue_3) (+ _output_get_y _returnvalue_3))))))

(event `EnhancedInput|/Game/InputSystem/Input_Zoom`
  (params (ActionValue :type "Float (double-precision)") (ElapsedSeconds :type "Float (double-precision)") (TriggeredSeconds :type "Float (double-precision)") (InputAction :type "InputAction Object Reference" :default "/Game/InputSystem/Input_Zoom.Input_Zoom"))
  (bind _returnvalue (`self.GetGridSize`))
  (:`Triggered`
    (`KismetSystemLibrary.PrintString` "Hello")
    (set `self.TargetZoom` (+ (`CameraComponent.OrthoWidth` (`self.Camera`)) (* ActionValue (* (`KismetMathLibrary.NormalizeToRange` (`CameraComponent.OrthoWidth` (`self.Camera`)) (/ _returnvalue 5.0) _returnvalue) (`self.ZoomIncrement`)))))))

(event `EnhancedInput|/Game/InputSystem/Input_Pan`
  (params (ActionValue :type "Vector2D Structure") (ElapsedSeconds :type "Float (double-precision)") (TriggeredSeconds :type "Float (double-precision)") (InputAction :type "InputAction Object Reference" :default "/Game/InputSystem/Input_Pan.Input_Pan"))
  (bind _movespeed (`self.MoveSpeed`))
  (bind (_x _y) (`KismetMathLibrary.BreakVector2D` (* ActionValue (`KismetMathLibrary.MakeVector2D` _movespeed _movespeed))))
  (bind (_returnvalue_x _returnvalue_y _returnvalue_z) (`KismetMathLibrary.BreakVector` (+ (`self.K2_GetActorLocation`) (`KismetMathLibrary.MakeVector` _y _x))))
  (:`Triggered`
    (set `self.bMoving` true)
    (set `self.TargetLocation` (`KismetMathLibrary.MakeVector` _returnvalue_x _returnvalue_y _returnvalue_z))
    (`KismetSystemLibrary.Delay` 0.8)
    (set `self.bMoving` false)))

(event `Key|SpaceBar`
  (params (Key :type "Key Structure"))
  (:`Pressed`
    (set `self.TargetLocation` (`self.GetGridCenter`))))

(fn `GetGridCenter`
  (returns (Output_Get :type "Vector Structure"))
  (bind _grid (`self.Grid`))
  (bind _grid_2 (`self.Grid`))
  (bind (_returnvalue_x _returnvalue_y _returnvalue_z) (`KismetMathLibrary.BreakVector` (`self.K2_GetActorLocation` (`self.Grid`))))
  (return (`KismetMathLibrary.MakeVector` (+ _returnvalue_x (* (* (`/Game/Blueprints/BP_GridGenerator.XSize` _grid_2) (`/Game/Blueprints/BP_GridGenerator.GridDistance` _grid_2)) 0.5)) (+ _returnvalue_y (* (* (`/Game/Blueprints/BP_GridGenerator.YSize` _grid) (`/Game/Blueprints/BP_GridGenerator.GridDistance` _grid)) 0.5)) _returnvalue_z)))

(fn `GetGridSize`
  (returns (ReturnValue :type "Float (double-precision)"))
  (bind _grid (`self.Grid`))
  (return (* (+ (* (`/Game/Blueprints/BP_GridGenerator.GridDistance` _grid) (`/Game/Blueprints/BP_GridGenerator.XSize` _grid)) (`self.Buffer`)) 2.0)))

(fn `UserConstructionScript`)